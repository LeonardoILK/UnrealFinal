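; BP_Trap is a puzzle trap that punishes the player for entering its box trigger.
; On overlap with the third-person character, it checks checkpoint state stored in the Time_DayNight game instance, cached on BeginPlay.
; With an active checkpoint, the player is moved to the last saved checkpoint transform; otherwise it sets the game-started flag and reloads the current level.
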(event OnComponentBeginOverlap(Box)
  (params (OverlappedComponent :type Primitive%20Component%20Object%20Reference) (OtherActor :type Actor%20Object%20Reference) (OtherComp :type Primitive%20Component%20Object%20Reference) (OtherBodyIndex :type Integer) (bFromSweep :type Boolean) (SweepResult :type Hit%20Result%20Structure%20%28by%20ref%29))
  (bind _giref (Variables|Default|GetGIRef))
  (Utilities|Casting|CastToBP_ThirdPersonCharacter OtherActor)
  (if (Variables|/Game/Puzzles/3_DayNight/GameInstance_Time_DayNight.GameInstance_Time_DayNight_C|GetGI_CheckpointActivated _giref)
    (Transformation|SetActorTransform (Game|GetPlayerCharacter 0) (Variables|/Game/Puzzles/3_DayNight/GameInstance_Time_DayNight.GameInstance_Time_DayNight_C|GetGI_Last_Checkpoint _giref))
    (else
      (Variables|/Game/Puzzles/3_DayNight/GameInstance_Time_DayNight.GameInstance_Time_DayNight_C|SetGI_GameStarted _giref true)
      (bind _returnvalue (Game|GetCurrentLevelName true))
      (Game|OpenLevel(byName) (Utilities|String|StringToName _returnvalue)))))

(event EventBeginPlay
  (bind _asgame_instance_time_day_night (Utilities|Casting|CastToGameInstance_Time_DayNight (Game|GetGameInstance)))
  (Variables|Default|SetGIRef _asgame_instance_time_day_night))

(fn ConstructionScript)
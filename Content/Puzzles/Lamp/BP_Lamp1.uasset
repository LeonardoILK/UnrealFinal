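; BP_Lamp1 is a puzzle-folder lamp with five point lights, switched by the third-person character entering and leaving a box trigger.
; On entry the main light turns on, occasionally flickering first, then TurnOn4Left loops over the other four with a short random Delay inside the loop.
; On exit, TurnOff waits a few seconds and hides all five, without checking whether the character has re-entered.
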(event OnComponentBeginOverlap(Box)
  (params (OverlappedComponent :type Primitive%20Component%20Object%20Reference) (OtherActor :type Actor%20Object%20Reference) (OtherComp :type Primitive%20Component%20Object%20Reference) (OtherBodyIndex :type Integer) (bFromSweep :type Boolean) (SweepResult :type Hit%20Result%20Structure%20%28by%20ref%29))
  (Utilities|Casting|CastToBP_ThirdPersonCharacter OtherActor)
  (if (>= (Math|Random|RandomFloatinRange 0.0 1.0) 0.8)
    (Rendering|SetVisibility (Variables|Default|GetPointLight) true false)
    (Utilities|FlowControl|Delay 0.1)
    (Rendering|SetVisibility (Variables|Default|GetPointLight) false false)
    (Utilities|FlowControl|Delay 0.1)
    (Rendering|SetVisibility (Variables|Default|GetPointLight) true false)
    (Utilities|FlowControl|Delay 0.1)
    (Rendering|SetVisibility (Variables|Default|GetPointLight) false false)
    (Utilities|FlowControl|Delay 0.1)
    (Rendering|SetVisibility (Variables|Default|GetPointLight) true false)
    (CallFunction|Turnon4Left)
    (else
      (Rendering|SetVisibility (Variables|Default|GetPointLight) true false)
      (CallFunction|Turnon4Left))))

(event OnComponentEndOverlap(Box)
  (params (OverlappedComponent :type Primitive%20Component%20Object%20Reference) (OtherActor :type Actor%20Object%20Reference) (OtherComp :type Primitive%20Component%20Object%20Reference) (OtherBodyIndex :type Integer))
  (Utilities|Casting|CastToBP_ThirdPersonCharacter OtherActor)
  (CallFunction|TurnOff))

(event Custom|TurnOff
  (Utilities|FlowControl|Delay 3.0)
  (for _array_element (Utilities|Array|MakeArray (Variables|Default|GetPointLight) (Variables|Default|GetPointLight1) (Variables|Default|GetPointLight2) (Variables|Default|GetPointLight3) (Variables|Default|GetPointLight4))
    (Rendering|SetVisibility _array_element false false)))

(event Custom|TurnOn4Left
  (Utilities|FlowControl|Delay 0.1)
  (for _array_element (Utilities|Array|MakeArray (Variables|Default|GetPointLight1) (Variables|Default|GetPointLight2) (Variables|Default|GetPointLight3) (Variables|Default|GetPointLight4))
    (Utilities|FlowControl|Delay (Math|Random|RandomFloatinRange 0.1 0.2))
    (Rendering|SetVisibility _array_element true false)))

(fn ConstructionScript)